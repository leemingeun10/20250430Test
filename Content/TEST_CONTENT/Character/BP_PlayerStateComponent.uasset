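; BP_PlayerStateComponent is an actor component that tracks the player wizard's health.
; On BeginPlay it sets current HP to max and starts a fast looping timer.
; The timer pushes the HP ratio to the HP tag in the owning BP_Wizard's HP widget component, polling rather than updating on change.
; UpdateCurHP simply overwrites current HP.
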(event EventBeginPlay
  (Variables|Default|SetCurHP (Variables|Default|GetMaxHP))
  (Utilities|Time|SetTimerbyFunctionName 0 "SetHptowidget" 0.05 true))

(event EventTick
  (params (DeltaSeconds :type Float%20%28single-precision%29)))

(fn UpdateCurHP
  (params (CurHP :type Float%20%28double-precision%29))
  (Variables|Default|SetCurHP CurHP))

(fn SetHptowidget
  (bind _asbp_wizard (Utilities|Casting|CastToBP_Wizard (Components|GetOwner)))
  (Default|UpdateHP (Variables|/Game/TEST_CONTENT/Character/BP_HPWidgetComponent.BP_HPWidgetComponent_C|GetHP_tag (Variables|/Game/TEST_CONTENT/Character/BP_Wizard.BP_Wizard_C|GetBP_HPWidgetComponent _asbp_wizard)) (/ (Variables|Default|GetCurHP) (Variables|Default|GetMaxHP))))