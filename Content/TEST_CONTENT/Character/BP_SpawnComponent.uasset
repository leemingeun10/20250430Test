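; Actor component that periodically spawns random monsters and boxes around its owner.
; A fast timer picks a point on a ring around the owner, checks for ground with a downward trace, then spawns a random DT_Monster AI running BT_Mon.
; MonArr stops monster spawning at ten entries and is never decremented here.
; A slower timer spawns random DT_Box actors at nearby navigable points, without a cap.
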(event EventBeginPlay
  (Utilities|Time|SetTimerbyFunctionName 0 "DoSpawn" 0.1 true)
  (Utilities|Time|SetTimerbyFunctionName 0 "DoSpawnBox" 3.0 true))

(event EventTick
  (params (DeltaSeconds :type Float%20%28single-precision%29)))

(fn DoSpawn
  (bind _monarr (Variables|Default|GetMonArr))
  (bind _returnvalue (Utilities|Array|Length _monarr))
  (bind _output_get (Variables|Default|SetRandomloc (CallFunction|MonspawnLoc)))
  (if (CallFunction|IsCanSpawnLoc _output_get)
    (if (not (or (> _returnvalue 10) (== _returnvalue 10)))
      (bind _outrownames (DataTable|GetDataTableRowNames "/Game/TEST_CONTENT/Monster/DT_Monster.DT_Monster"))
      (Utilities|Array|Add (Variables|Default|GetMonArr) (.OutItem (Utilities|Array|Random _outrownames)))
      (bind _returnvalue_2 (Utilities|GetDataTableRow "/Game/TEST_CONTENT/Monster/DT_Monster.DT_Monster" (.OutItem (Utilities|Array|Random _outrownames)))
        (:then
          (AI|SpawnAIFromClass (.monster (Utilities|Struct|BreakST_Monster _returnvalue_2)) "/Game/TEST_CONTENT/AI/BT_Mon.BT_Mon" (Variables|Default|GetRandomloc) "0, 0, 0" false 0))))))

(fn MonspawnLoc
  (bind _radius (Variables|Default|GetRadius))
  (bind _returnvalue (* _radius 3.141592))
  (bind _output_get (LocalVariables|Setvar (Math|Random|RandomFloatinRange 0.0 3.6e+02)))
  (return (+ (Transformation|GetActorLocation (Components|GetOwner)) (Math|Vector|MakeVector (* (Math|Trig|Cos(Radians) _output_get) _returnvalue) (* (Math|Trig|Sin(Radians) _output_get) _returnvalue) 0.0))))

(fn IsCanSpawnLoc
  (params (worldLocation :type Vector))
  (bind _returnvalue (Collision|LineTraceForObjects worldLocation (- worldLocation "0.000000,0.000000,100.000000") (Utilities|Array|MakeArray "ObjectTypeQuery1" "ObjectTypeQuery2") false 0 "None"))
  (return _returnvalue))

(fn DoSpawnBox
  (bind _outrownames (DataTable|GetDataTableRowNames "/Game/TEST_CONTENT/Boxes/DT_Box.DT_Box"))
  (bind _output_get (Variables|Default|SetBox (.OutItem (Utilities|Array|Random _outrownames))))
  (bind _returnvalue (Utilities|GetDataTableRow "/Game/TEST_CONTENT/Boxes/DT_Box.DT_Box" _output_get)
    (:then
      (bind _randomlocation (Class|NavigationSystemV1|GetRandomLocationinNavigableRadius (Transformation|GetActorLocation (Components|GetOwner)) 5e+02 0 0))
      (Game|SpawnActorfromClass (.Box (Utilities|Struct|BreakST_Box _returnvalue)) (Math|Conversions|ToTransform(Vector) _randomlocation) "Undefined" "MultiplyWithRoot" 0 0))))